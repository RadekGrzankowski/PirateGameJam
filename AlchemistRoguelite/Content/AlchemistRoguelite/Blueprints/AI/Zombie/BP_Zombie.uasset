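; Zombie melee enemy that follows the player from BeginPlay and attacks when able.
; Each Tick runs CanAttack, then stops CharacterMovement and alternates two attack montages via the AttackChange flag, reactivating movement when each completes.
; MeeleDamagePlayer deals damage only if the player is within AttackRange plus the AttackRangeFixed offset; nothing in these graphs calls it.
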(event `self.ReceiveBeginPlay`
  (`/Game/AlchemistRoguelite/Blueprints/Macros/MyMacros.FollowPlayer`))

(event `self.ReceiveTick`
  (params (DeltaSeconds :type "Float (single-precision)"))
  (bind _mesh (`self.Mesh`))
  (bind _charactermovement (`self.CharacterMovement`))
  (if (`/Game/AlchemistRoguelite/Blueprints/Macros/MyMacros.CanAttack` (`self.IsAlive`) (`self.AttackRange`) "/Game/UndeadPack/Zombie/Animations/ZombieAttack1.ZombieAttack1" "/Game/UndeadPack/Zombie/Animations/ZombieAttack2.ZombieAttack2" (`self.Mesh`))
    (`ActorComponent.Deactivate` (`self.CharacterMovement`))
    (if (`self.AttackChange`)
      (`|PlayMontage` _mesh "/Game/UndeadPack/Zombie/Animations/ZombieAttack1.ZombieAttack1"
        (:`then`
          (set `self.AttackChange` false))
        (:`OnCompleted`
          (`ActorComponent.Activate` _charactermovement false)))
      (else
        (`|PlayMontage` _mesh "/Game/UndeadPack/Zombie/Animations/ZombieAttack2.ZombieAttack2"
          (:`then`
            (set `self.AttackChange` true))
          (:`OnCompleted`
            (`ActorComponent.Activate` _charactermovement false)))))))

(fn `IsWithinFixedAttackRange`
  (returns (ReturnValue :type Boolean))
  (return (< (`self.GetDistanceTo` (`GameplayStatics.GetPlayerCharacter` 0)) (+ (`self.AttackRange`) (`self.AttackRangeFixed`)))))

(fn `MeeleDamagePlayer`
  (if (`self.IsWithinFixedAttackRange`)
    (`/Game/AlchemistRoguelite/Blueprints/Macros/MyMacros.DamagePlayer` (`self.MeeleDamage`))))

(fn `UserConstructionScript`)