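; Melee goblin enemy that follows the player from spawn and attacks when in range.
; Each tick a CanAttack check gates the attack, which stops movement and alternates two montages, re-enabling movement when the montage completes.
; A separate damage function, not called within this graph, hurts the player only within an extended attack range.
; Incoming damage reduces clamped, normalized health and destroys the goblin at zero.
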(event `self.ReceiveBeginPlay`
  (`/Game/AlchemistRoguelite/Blueprints/Macros/MyMacros.FollowPlayer`))

(event `self.ReceiveTick`
  (params (DeltaSeconds :type "Float (single-precision)"))
  (bind _mesh (`self.Mesh`))
  (bind _charactermovement (`self.CharacterMovement`))
  (if (`/Game/AlchemistRoguelite/Blueprints/Macros/MyMacros.CanAttack` (`self.IsAlive?`) (`self.AttackRange`) "/Game/UndeadPack/EnemyGoblin/Animations/GoblinAttack1.GoblinAttack1" "/Game/UndeadPack/EnemyGoblin/Animations/GoblinAttack2.GoblinAttack2" (`self.Mesh`))
    (`ActorComponent.Deactivate` (`self.CharacterMovement`))
    (if (`self.AttackChange`)
      (`|PlayMontage` _mesh "/Game/UndeadPack/EnemyGoblin/Animations/GoblinAttack1.GoblinAttack1"
        (:`then`
          (set `self.AttackChange` false))
        (:`OnCompleted`
          (`ActorComponent.Activate` _charactermovement false)))
      (else
        (`|PlayMontage` _mesh "/Game/UndeadPack/EnemyGoblin/Animations/GoblinAttack2.GoblinAttack2"
          (:`then`
            (set `self.AttackChange` true))
          (:`OnCompleted`
            (`ActorComponent.Activate` _charactermovement false)))))))

(event `self.ReceiveAnyDamage`
  (params (Damage :type "Float (single-precision)") (DamageType :type "DamageType Object Reference") (InstigatedBy :type "Controller Object Reference") (DamageCauser :type "Actor Object Reference"))
  (bind _output_get (set `self.Health` (`KismetMathLibrary.FClamp` (- (`self.Health`) Damage))))
  (if (<= _output_get 0.0)
    (`self.K2_DestroyActor`)))

(fn `IsWithinFixedAttackRange`
  (returns (ReturnValue :type Boolean))
  (return (< (`self.GetDistanceTo` (`GameplayStatics.GetPlayerCharacter` 0)) (+ (`self.AttackRange`) (`self.AttackRangeFixed`)))))

(fn `MeeleDamagePlayer`
  (if (`self.IsWithinFixedAttackRange`)
    (`/Game/AlchemistRoguelite/Blueprints/Macros/MyMacros.DamagePlayer` (`self.MeeleDamage`))))

(fn `UserConstructionScript`)