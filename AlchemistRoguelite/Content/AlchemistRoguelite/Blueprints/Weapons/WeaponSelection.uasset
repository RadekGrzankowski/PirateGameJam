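; WeaponSelection is an actor that handles weapon pickups, offering a choice of weapon through a selection widget.
; It creates the widget on BeginPlay; overlapping a WeaponPickUp destroys the pickup, sets a flag, pauses the game and shows the widget.
; While flagged, Tick converts the widget's choice to a WeaponArray index and spawns that class at this actor's transform after a short delay.
; The flag is never cleared here, so spawning can repeat.
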(event `self.ReceiveBeginPlay`
  (bind _returnvalue (`|CreateWidget` "/Game/AlchemistRoguelite/UI/WBP_WeaponSelection.WBP_WeaponSelection_C"))
  (set `self.WBP WeaponSelectionRef` _returnvalue))

(event `self.ReceiveActorBeginOverlap`
  (params (OtherActor :type "Actor Object Reference"))
  (bind _asweapon_pick_up (cast `/Game/AlchemistRoguelite/Blueprints/PickUps/WeaponPickUp` OtherActor))
  (`/Engine/EditorBlueprintResources/StandardMacros.IsValid` _asweapon_pick_up
    (:`Is Valid`
      (set `self.WeaponPickedUp` true)
      (`self.K2_DestroyActor` _asweapon_pick_up)
      (`GameplayStatics.SetGamePaused` true)
      (`UserWidget.AddToViewport` (`self.WBP WeaponSelectionRef`) 0))))

(event `self.ReceiveTick`
  (params (DeltaSeconds :type "Float (single-precision)"))
  (if (`self.WeaponPickedUp`)
    (bind _output_get (set `self.WeaponChoice` (`/Game/AlchemistRoguelite/UI/WBP_WeaponSelection.WeaponChoice` (`self.WBP WeaponSelectionRef`))))
    (bind _result (`/Engine/EditorBlueprintResources/StandardMacros.DecrementInt` _output_get)
      (:`  `
        (for (_ _array_index) (`self.WeaponArray`)
          (if (== _array_index _result)
            (`KismetSystemLibrary.Delay` 0.5)
            (`|SpawnActorFromClass` (`|GetArrayItem` (`self.WeaponArray`) _result) (`KismetMathLibrary.MakeTransform` (`self.K2_GetActorLocation` self) (`self.K2_GetActorRotation` self)) "Undefined" "SelectDefaultAtRuntime" null null)))))))

(fn `UserConstructionScript`)